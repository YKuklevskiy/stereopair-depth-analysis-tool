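; Robot3_BP is a drivable robot vehicle pawn with throttle, brake, steering, handbrake and mouse look.
; Input events feed the vehicle movement component directly, with negative forward input converted to brake.
; On BeginPlay, InitialSetup loads JSON through a reader component and reads wheel radius, camera offset and arm height offset, but does not apply them.
; A HUD texture draw is left unconnected and never runs.
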(event `self.ReceiveBeginPlay`
  (`self.InitialSetup`))

(event `self.ReceiveTick`
  (params (DeltaSeconds :type "Float (single-precision)")))

(event `InputAxis|Look Up`
  (params (AxisValue :type "Float (single-precision)"))
  ;[1 1 1] MouseControls
  (`self.AddControllerPitchInput` AxisValue))

(event `InputAxis|Look Right`
  (params (AxisValue :type "Float (single-precision)"))
  ;[1 1 1] MouseControls
  (`self.AddControllerYawInput` AxisValue))

(event `InputAction|Handbrake`
  (params (Key :type "Key Structure"))
  (bind _vehiclemovementcomponent (`self.VehicleMovementComponent`))
  ;[1 1 1] HandbrakeControls
  (:`Pressed`
    (`ChaosVehicleMovementComponent.SetHandbrakeInput` _vehiclemovementcomponent true))
  (:`Released`
    (`ChaosVehicleMovementComponent.SetHandbrakeInput` _vehiclemovementcomponent false)))

(event `InputAxis|Move Forward`
  (params (AxisValue :type "Float (single-precision)"))
  (bind _vehiclemovementcomponent (`self.VehicleMovementComponent`))
  ;[1 1 1] Throttle & Break Controls
  (if (>= AxisValue 0.0)
    (`ChaosVehicleMovementComponent.SetThrottleInput` _vehiclemovementcomponent AxisValue)
    (`ChaosVehicleMovementComponent.SetBrakeInput` _vehiclemovementcomponent 0.0)
    (else
      (`ChaosVehicleMovementComponent.SetBrakeInput` _vehiclemovementcomponent (* AxisValue -1.0))
      (`ChaosVehicleMovementComponent.SetThrottleInput` _vehiclemovementcomponent 0.0))))

(event `InputAxis|Move Right`
  (params (AxisValue :type "Float (single-precision)"))
  ;[1 1 1] TurnControls
  (`ChaosVehicleMovementComponent.SetSteeringInput` (`self.VehicleMovementComponent`) AxisValue))

(fn `InitialSetup`
  (bind _jsonreadercomponent (`self.JSONReaderComponent`))
  (`/Game/JSONReaderComponent.LoadJSON` _jsonreadercomponent)
  (`/Game/JSONReaderComponent.GetFloat` _jsonreadercomponent "wheel radius")
  (`/Game/JSONReaderComponent.GetFloatArray` _jsonreadercomponent "camera offset")
  (`/Game/JSONReaderComponent.GetFloat` _jsonreadercomponent "arm height offset"))

(fn `UserConstructionScript`)